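; Level-end Blueprint that puts the ResultsUI widget on screen when the level finishes.
; Every Tick, while Good is set, it compares the EnemyData count from the MapData actor to KillCount and shows results if they match and LevelEnd is true.
; When Good is false, it shows results directly.
; Neither path has a once-only guard, so a new widget is added each frame its conditions hold.
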(event EventTick
  (params (DeltaSeconds :type Float%20%28single-precision%29))
  (if (Variables|Default|GetGood)
    (bind _returnvalue (Actor|GetActorOfClass "/Game/MapData/MapData.MapData_C"))
    (if (== (Utilities|Array|Length (Variables|/Game/MapData/MapData.MapData_C|GetEnemyData _returnvalue)) (Variables|Default|GetKillCount))
      (if (Variables|Default|GetLevelEnd)
        (bind _returnvalue_2 (UserInterface|CreateWidget "/Game/UIStuff/ResultsUI.ResultsUI_C"))
        (UserInterface|Viewport|AddtoViewport _returnvalue_2 0)))
    (else
      (bind _returnvalue_3 (UserInterface|CreateWidget "/Game/UIStuff/ResultsUI.ResultsUI_C"))
      (UserInterface|Viewport|AddtoViewport _returnvalue_3 0))))

(fn ConstructionScript)