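; Player pointer actor that turns each tick toward the mouse's angle around the world origin and kills enemies by matching keys.
; Key presses are filtered to W/A/S/D as CurrentKey; an enemy touching Tip is rechecked via a delay loop until its IKillKey matches or it becomes invalid.
; DeathArea destroys overlapping actors and costs a Health life; both kill paths increment LevelEnd's KillCount.
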(event OnComponentBeginOverlap(Tip)
  (params (OverlappedComponent :type Primitive%20Component%20Object%20Reference) (OtherActor :type Actor%20Object%20Reference) (OtherComp :type Primitive%20Component%20Object%20Reference) (OtherBodyIndex :type Integer) (bFromSweep :type Boolean) (SweepResult :type Hit%20Result%20Structure%20%28by%20ref%29))
  (bind _output_get (Variables|Default|SetCurrentEnemy OtherActor))
  (bind _asenemy (Utilities|Casting|CastToEnemy _output_get))
  (if (Utilities|Enum|Equal(Enum) (Variables|/Game/Blueprints/Enemy.Enemy_C|GetIKillKey _asenemy) (Variables|Default|GetCurrentKey)) :!label _label
    (Utilities|IsValid (Variables|Default|GetCurrentEnemy)
      (:Is%20Valid
        (Actor|DestroyActor (Variables|Default|GetCurrentEnemy))
        (bind _returnvalue (Actor|GetActorOfClass "/Game/Blueprints/levelEnd.levelEnd_C"))
        (Variables|/Game/Blueprints/levelEnd.levelEnd_C|SetKillCount _returnvalue (+ (Variables|/Game/Blueprints/levelEnd.levelEnd_C|GetKillCount _returnvalue) 1))))
    (else
      (Utilities|FlowControl|Delay (Utilities|Time|GetWorldDeltaSeconds))
      (Utilities|IsValid (Variables|Default|GetCurrentEnemy)
        (:Is%20Valid
          (goto _label))))))

(event OnComponentBeginOverlap(DeathArea)
  (params (OverlappedComponent :type Primitive%20Component%20Object%20Reference) (OtherActor :type Actor%20Object%20Reference) (OtherComp :type Primitive%20Component%20Object%20Reference) (OtherBodyIndex :type Integer) (bFromSweep :type Boolean) (SweepResult :type Hit%20Result%20Structure%20%28by%20ref%29))
  (Actor|DestroyActor OtherActor)
  (bind _returnvalue (Actor|GetActorOfClass "/Game/Blueprints/Health.Health_C"))
  (Variables|/Game/Blueprints/Health.Health_C|Setlives _returnvalue (- (Variables|/Game/Blueprints/Health.Health_C|Getlives _returnvalue) 1.0))
  (bind _returnvalue_2 (Actor|GetActorOfClass "/Game/Blueprints/levelEnd.levelEnd_C"))
  (Variables|/Game/Blueprints/levelEnd.levelEnd_C|SetKillCount _returnvalue_2 (+ (Variables|/Game/Blueprints/levelEnd.levelEnd_C|GetKillCount _returnvalue_2) 1)))

(event EventTick
  (params (DeltaSeconds :type Float%20%28single-precision%29))
  (bind _degree (CallFunction|SetRot))
  (Transformation|SetActorRotation (Math|Rotator|MakeRotator 0.0 0.0 (Utilities|ToZRot _degree))))

(event Input|KeyboardEvents|AnyKey
  (params (Key :type Key%20Structure :default "None"))
  (:Pressed
    (bind _output (CallFunction|NewFunction0 (Utilities|KeytoString Key)))
    (Variables|Default|SetCurrentKey _output)))

(fn ConstructionScript)

(fn SetRot
  (bind _returnvalue (Game|GetPlayerController 0))
  (bind _worldlocation (Game|Player|ConvertMouseLocationToWorldSpace _returnvalue))
  (bind _returnvalue_2 (Class|KismetMathLibrary|DegAtan2 (.y _worldlocation) (.x _worldlocation)))
  (bind _returnvalue_3 (- _returnvalue_2 9e+01))
  (bind _returnvalue_4 (* _returnvalue_3 -1.0))
  (if (<= _returnvalue_4 0.0)
    (return (+ _returnvalue_4 3.6e+02))
    (else
      (return _returnvalue_4))))

(fn NewFunction0
  (params (Input :type String))
  (if (not (and (and (Utilities|Enum|NotEqual(Enum) Input "W") (Utilities|Enum|NotEqual(Enum) Input "A")) (and (Utilities|Enum|NotEqual(Enum) Input "S") (Utilities|Enum|NotEqual(Enum) Input "D"))))
    (return Input)))