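; Enemy actor that moves toward the world origin and is killed by the pointer's tip when the matching key is active.
; On BeginPlay it copies speed and kill key from MapData, whose material index also picks its mesh material and key label.
; Tick advances it at constant speed via VInterpToConstant.
; Capsule overlap with Pointer_Blueprint's Tip checks the current key, then increments LevelEnd's KillCount and destroys the enemy.
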(event OnComponentBeginOverlap(Capsule)
  (params (OverlappedComponent :type Primitive%20Component%20Object%20Reference) (OtherActor :type Actor%20Object%20Reference) (OtherComp :type Primitive%20Component%20Object%20Reference) (OtherBodyIndex :type Integer) (bFromSweep :type Boolean) (SweepResult :type Hit%20Result%20Structure%20%28by%20ref%29))
  (bind _returnvalue (Actor|GetActorOfClass "/Game/Blueprints/Pointer_Blueprint.Pointer_Blueprint_C"))
  (if (and (== (Variables|/Game/Blueprints/Pointer_Blueprint.Pointer_Blueprint_C|GetTip _returnvalue) OtherComp) (Utilities|Enum|Equal(Enum) (Variables|Default|GetIkillKey) (Variables|/Game/Blueprints/Pointer_Blueprint.Pointer_Blueprint_C|GetCurrentKey _returnvalue)))
    (bind _returnvalue_2 (Actor|GetActorOfClass "/Game/Blueprints/levelEnd.levelEnd_C"))
    (Variables|/Game/Blueprints/levelEnd.levelEnd_C|SetKillCount _returnvalue_2 (+ (Variables|/Game/Blueprints/levelEnd.levelEnd_C|GetKillCount _returnvalue_2) 1))
    (Actor|DestroyActor)))

(event EventBeginPlay
  (bind _returnvalue (Actor|GetActorOfClass "/Game/SpawnData/MapData.MapData_C"))
  (Variables|Default|SetISpeed (Variables|/Game/SpawnData/MapData.MapData_C|GetSpeed _returnvalue))
  (Variables|Default|SetIkillKey (Variables|/Game/SpawnData/MapData.MapData_C|GetKillKey _returnvalue))
  (Rendering|Material|SetMaterial (Variables|Debug|GetStaticMeshComponent) 0 (Utilities|Array|Get(acopy) (Variables|Default|GetContainer) (Variables|/Game/SpawnData/MapData.MapData_C|GetMaterial _returnvalue)))
  (Rendering|Components|TextRender|SetText (Variables|Default|GetTextRender) (Utilities|Array|Get(acopy) (Variables|Default|GetKeyHolder) (Variables|/Game/SpawnData/MapData.MapData_C|GetMaterial _returnvalue))))

(event EventTick
  (params (DeltaSeconds :type Float%20%28single-precision%29))
  (CallFunction|MovetoOrigin))

(fn ConstructionScript)

(fn MovetoOrigin
  (Transformation|SetActorLocation (Math|Interpolation|VInterptoConstant (Transformation|GetActorLocation) "0, 0, 0" (Utilities|Time|GetWorldDeltaSeconds) (Variables|Default|GetISpeed)) false false))